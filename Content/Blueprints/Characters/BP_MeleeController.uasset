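; BP_MeleeController is an AI controller for melee characters that runs the BT_Melee behavior tree on possession.
; Every tick it writes the player character into the Blackboard as the target actor.
; It binds to the melee anim instance's OnApplyDamage event, so the animation times the hit.
; That event makes the pawn's BP_WeaponComponent, if valid, attack the Blackboard target.
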(event `self.ReceiveBeginPlay`
  (add `/Game/Animations/Enemies/ABP_Melee.OnApplyDamage` (`/Game/Blueprints/Components/BP_MeleeAnimComponent.GetMeleeAnimInstance` (`self.MeleeAnimComponent`)) (delegate `OnApplyDamage`)))

(event `OnApplyDamage`
  (`self.AttackTarget`))

(event `self.ReceiveTick`
  (params (DeltaSeconds :type "Float (single-precision)"))
  (`BlackboardComponent.SetValueAsObject` (`self.Blackboard`) (`self.TargetActorKeyName`) (`GameplayStatics.GetPlayerCharacter` 0)))

(event `self.ReceivePossess`
  (params (PossessedPawn :type "Pawn Object Reference"))
  (`self.RunBehaviorTree` "/Game/Blueprints/Characters/BT_Melee.BT_Melee"))

(fn `AttackTarget`
  (bind _returnvalue (`self.GetComponentByClass` (`self.K2_GetPawn`) "/Game/Blueprints/Components/BP_WeaponComponent.BP_WeaponComponent_C"))
  (`/Engine/EditorBlueprintResources/StandardMacros.IsValid` _returnvalue
    (:`Is Valid`
      (`/Game/Blueprints/Components/BP_WeaponComponent.AttackActor` _returnvalue (`self.GetTargetActor`)))))

(fn `GetTargetActor`
  (returns (TargetActor :type "Actor Object Reference"))
  (bind _asactor (cast `Actor` (`BlackboardComponent.GetValueAsObject` (`self.Blackboard`) (`self.TargetActorKeyName`)))
    (:`then`
      (return _asactor))
    (:`CastFailed`
      (return null))))

(fn `UserConstructionScript`)