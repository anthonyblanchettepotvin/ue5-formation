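; BP_Player is the player character Blueprint, handling a world-space cursor and damage-driven death.
; Each tick, it traces under the mouse cursor on the Visibility channel and moves CursorToWorld to the hit location, oriented along the surface normal.
; Any damage received is subtracted through HealthComponent's RemoveLife, and the component's OnDie event destroys the actor.
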(event `self.ReceiveTick`
  (params (DeltaSeconds :type "Float (single-precision)"))
  (bind (_bblockinghit _binitialoverlap _time _distance _location _impactpoint _normal _impactnormal) (`GameplayStatics.BreakHitResult` (`PlayerController.GetHitResultUnderCursorByChannel` (`GameplayStatics.GetPlayerController` 0) "TraceTypeQuery1" true)))
  (`SceneComponent.K2_SetWorldLocationAndRotation` (`self.CursorToWorld`) _location (`KismetMathLibrary.MakeRotationFromAxes` _impactnormal) false false))

(event `self.ReceiveAnyDamage`
  (params (Damage :type "Float (single-precision)") (DamageType :type "DamageType Object Reference") (InstigatedBy :type "Controller Object Reference") (DamageCauser :type "Actor Object Reference"))
  (`/Game/Blueprints/Components/BP_HealthComponent.RemoveLife` (`self.HealthComponent`) Damage))

(event `self.HealthComponent.OnDie`
  (`self.K2_DestroyActor`))

(fn `UserConstructionScript`)