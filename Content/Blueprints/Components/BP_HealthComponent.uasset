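; Health component that tracks an actor's current and maximum life and handles healing, damage and death.
; AddLife and RemoveLife clamp the result between zero and the maximum, and both do nothing once life is zero, so healing cannot revive.
; Changes fire the OnLifeChanged dispatcher, and damage that empties life also fires OnDie.
; Helper functions report death, missing life and life as a fraction of maximum.
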(fn `AddLife`
  (params (Amount :type "Float (double-precision)"))
  (if (not (`self.IsDead`))
    (if (> Amount (`self.GetMissingLife`))
      (set `self.CurrentLife` (`self.MaximumLife`))
      (else
        (set `self.CurrentLife` (+ Amount (`self.CurrentLife`)))))
    (`self.OnLifeChanged`)))

(fn `GetMissingLife`
  (returns (MissingLife :type "Float (double-precision)"))
  (return (- (`self.MaximumLife`) (`self.CurrentLife`))))

(fn `GetPercentLife`
  (returns (PercentLife :type "Float (double-precision)"))
  (return (/ (`self.CurrentLife`) (`self.MaximumLife`))))

(fn `IsDead`
  (returns (IsDead :type Boolean))
  (return (== (`self.CurrentLife`) 0.0)))

(fn `RemoveLife`
  (params (Amount :type "Float (double-precision)"))
  (if (not (`self.IsDead`))
    (if (> Amount (`self.CurrentLife`))
      (set `self.CurrentLife` 0.0)
      (else
        (set `self.CurrentLife` (- (`self.CurrentLife`) Amount))))
    (`self.OnLifeChanged`)
    (if (`self.IsDead`)
      (`self.OnDie`))))