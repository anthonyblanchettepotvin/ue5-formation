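; Controller component that bridges to the melee animation Blueprint of the controlled pawn.
; It resolves ABP_Melee by casting its owning Controller's pawn to Character and reading the mesh's anim instance.
; IsAttacking reports that instance's attack state, defaulting to false, and NotifyShouldAttack forwards an attack request to it, both guarded by validity checks.
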(fn `GetMeleeAnimInstance`
  (returns (MeleeAnimInstance :type "/Game/Animations/Enemies/ABP_Melee Object Reference"))
  (bind _ascontroller (cast `Controller` (`self.GetOwner`)))
  (bind _ascharacter (cast `Character` (`Controller.K2_GetPawn` _ascontroller)))
  (bind _asabp_melee (cast `/Game/Animations/Enemies/ABP_Melee` (`SkeletalMeshComponent.GetAnimInstance` (`Character.Mesh` _ascharacter))))
  (return _asabp_melee))

(fn `IsAttacking`
  (returns (IsAttacking :type Boolean))
  (bind _meleeaniminstance (`self.GetMeleeAnimInstance`))
  (`/Engine/EditorBlueprintResources/StandardMacros.IsValid` _meleeaniminstance
    (:`Is Valid`
      (return (`/Game/Animations/Enemies/ABP_Melee.IsAttacking` _meleeaniminstance)))
    (:`Is Not Valid`
      (return false))))

(fn `NotifyShouldAttack`
  (bind _meleeaniminstance (`self.GetMeleeAnimInstance`))
  (`/Engine/EditorBlueprintResources/StandardMacros.IsValid` _meleeaniminstance
    (:`Is Valid`
      (`/Game/Animations/Enemies/ABP_Melee.NotifyShouldAttack` _meleeaniminstance))))